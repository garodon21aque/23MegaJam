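; BP_Gas_Panel is an interactable gas panel that switches the level's fans on or off.
; On interaction, if the player holds the repair tool and IsGasFull is set, HasLec decides between StartFan and StopFan.
; Both events call every BP_Fan in the level, with loop bounds from -1 to the array length.
; A looping timer checks HasLec but does nothing, and LookAt returns an empty message.
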(event `self.ReceiveBeginPlay`
  (`KismetSystemLibrary.K2_SetTimerDelegate` (delegate `CustomEvent`) 1.0 true))

(event `CustomEvent`
  (if (`self.HasLec`)
    _))

(event `self.ReceiveTick`
  (params (DeltaSeconds :type "Float (single-precision)")))

(event `/Game/Blueprints/Interaction/BP_InteractionIF.InteractWith`
  (params (PC :type "/Game/FirstPerson/Blueprints/BP_FirstPersonCharacter Object Reference"))
  (bind _asbp_first_person_character (cast `/Game/FirstPerson/Blueprints/BP_FirstPersonCharacter` (`GameplayStatics.GetPlayerCharacter` 0)))
  (if (`/Game/FirstPerson/Blueprints/BP_FirstPersonCharacter.HasRepairTool` _asbp_first_person_character)
    (if (`self.IsGasFull`)
      (if (`self.HasLec`)
        (`self.StartFan`)
        (else
          (`self.StopFan`))))))

(event `StartFan`
  (bind _outactors (`GameplayStatics.GetAllActorsOfClass` "/Game/Blueprints/Actors/BP_Fan.BP_Fan_C"))
  (for _index (range -1 (+ (`KismetArrayLibrary.Array_Length` _outactors) 1))
    (`/Game/Blueprints/Actors/BP_Fan.StartFan1` (`|GetArrayItem` _outactors _index))))

(event `StopFan`
  (bind _outactors (`GameplayStatics.GetAllActorsOfClass` "/Game/Blueprints/Actors/BP_Fan.BP_Fan_C"))
  (for _index (range -1 (+ (`KismetArrayLibrary.Array_Length` _outactors) 1))
    (`/Game/Blueprints/Actors/BP_Fan.StopFan1` (`|GetArrayItem` _outactors _index))))

(fn `LookAt`
  (returns (Message :type Text) (Player :type "/Game/FirstPerson/Blueprints/BP_FirstPersonCharacter Object Reference"))
  (return "" null))

(fn `UserConstructionScript`)