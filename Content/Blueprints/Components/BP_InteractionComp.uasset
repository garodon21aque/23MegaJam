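; Interaction component that detects what the player camera is looking at and lets the player interact with it.
; Every tick a sphere trace from the camera stores the hit actor, or clears it on a miss, and prints the LookAtMessage text of actors implementing BP_InteractionIF.
; The Interact input sends InteractWithMessage to the stored actor.
; Disconnected nodes hold unfinished custom-depth highlight logic that never runs.
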(event `self.ReceiveBeginPlay`)

(event `self.ReceiveTick`
  (params (DeltaSeconds :type "Float (single-precision)"))
  (`self.InteractionTrace`))

(event `InputAction|Interact`
  (params (Key :type "Key Structure"))
  (:`Pressed`
    (message `/Game/Blueprints/Interaction/BP_InteractionIF.InteractWith` (`self.InteractActor`) null)))

(fn `InteractionTrace`
  (locals (LOCHResults :type "HitResult Structure"))
  (bind _returnvalue (`GameplayStatics.GetPlayerCameraManager` 0))
  (bind _returnvalue_2 (`Actor.K2_GetActorLocation` _returnvalue))
  (bind (_outhit _returnvalue_3) (`KismetSystemLibrary.SphereTraceSingle` _returnvalue_2 (+ _returnvalue_2 (* (`Actor.GetActorForwardVector` _returnvalue) (`self.TraceDistance`))) 20.0 "TraceTypeQuery3" false (`|MakeArray` (`self.GetOwner`))))
  (if _returnvalue_3
    (bind (_bblockinghit _binitialoverlap _time _distance _location _impactpoint _normal _impactnormal _physmat _hitactor) (`GameplayStatics.BreakHitResult` _outhit))
    (set `self.InteractActor` _hitactor)
    (if (`KismetSystemLibrary.DoesImplementInterface` _hitactor "/Game/Blueprints/Interaction/BP_InteractionIF.BP_InteractionIF_C")
      (bind _message (message `/Game/Blueprints/Interaction/BP_InteractionIF.LookAt` (`self.InteractActor`)))
      (`KismetSystemLibrary.PrintString` (`KismetTextLibrary.Conv_TextToString` _message)))
    (else
      (set `self.InteractActor` null))))