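; Sliding door actor that opens and closes through its OpenDoor and CloseDoor events.
; Each event adds an FMOD audio component and runs its own timeline, forward to open or reversed from the end to close, moving the Door along relative Y with sweep.
; Timeline updates also set the IsOpen flag.
; LookAt returns an empty message.
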(event `OpenDoor`
  (bind (_relativelocation_x _relativelocation_y _relativelocation_z) (`KismetMathLibrary.BreakVector` (`SceneComponent.RelativeLocation` (`self.Door`))))
  (`AddComponent|NODE_AddFMODAudioComponent-0`)
  (bind (_direction _open) (`Timeline|Timeline` :!via `PlayFromStart`)
    (:`Update`
      (`SceneComponent.K2_SetRelativeLocation` (`self.Door`) (`KismetMathLibrary.MakeVector` _relativelocation_x _open _relativelocation_z) true false)
      (set `self.IsOpen` true))))

(event `CloseDoor`
  (bind (_relativelocation_x _relativelocation_y _relativelocation_z) (`KismetMathLibrary.BreakVector` (`SceneComponent.RelativeLocation` (`self.Door`))))
  (`AddComponent|NODE_AddFMODAudioComponent-1`)
  (bind (_direction _open) (`Timeline|Timeline_0` :!via `ReverseFromEnd`)
    (:`Update`
      (`SceneComponent.K2_SetRelativeLocation` (`self.Door`) (`KismetMathLibrary.MakeVector` _relativelocation_x _open _relativelocation_z) true false)
      (set `self.IsOpen` false))))

(fn `LookAt`
  (returns (Message :type Text) (Player :type "/Game/FirstPerson/Blueprints/BP_FirstPersonCharacter Object Reference"))
  (return "" null))

(fn `UserConstructionScript`)