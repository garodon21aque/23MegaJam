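; BP_LampPoint is a lamp actor whose point light flickers on and off from BeginPlay.
; StartFlickering sets a looping timer that fires Flickering, which zeroes the intensity, waits a random delay, then restores it.
; StopFlickering only restores full intensity and leaves the timer running, so the flicker continues afterwards.
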(event `self.ReceiveBeginPlay`
  (`self.StartFlickering`))

(event `StartFlickering`
  (`KismetSystemLibrary.K2_SetTimerDelegate` (delegate `Flickering`) 1.5 true))

(event `Flickering`
  (`LightComponent.SetIntensity` (`self.PointLight`) 0.0)
  (`KismetSystemLibrary.Delay` (`KismetMathLibrary.RandomFloatInRange` 1.0 2.0))
  (`LightComponent.SetIntensity` (`self.PointLight`) 50.0))

(event `StopFlickering`
  (`LightComponent.SetIntensity` (`self.PointLight`) 50.0))

(fn `UserConstructionScript`)