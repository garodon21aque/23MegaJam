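; BP_Poison is a poison hazard actor that damages the first-person player character on overlapping its box, while its Poison component is active.
; Entry subtracts health immediately, then shows the WBP_Death widget with UI-only input and cursor if health is depleted.
; Otherwise, a single delayed follow-up hit lands and prints the remaining health, without checking again for death or overlap.
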(event `self.Box.OnComponentBeginOverlap`
  (params (OverlappedComponent :type "PrimitiveComponent Object Reference") (OtherActor :type "Actor Object Reference") (OtherComp :type "PrimitiveComponent Object Reference") (OtherBodyIndex :type Integer) (bFromSweep :type Boolean) (SweepResult :type "HitResult Structure (by ref)"))
  (bind _returnvalue (`GameplayStatics.GetPlayerController` 0))
  (bind _asbp_first_person_character (cast `/Game/FirstPerson/Blueprints/BP_FirstPersonCharacter` OtherActor))
  (if (`ActorComponent.IsActive` (`self.Poison`))
    (bind _health (`/Game/FirstPerson/Blueprints/BP_FirstPersonCharacter.Health` _asbp_first_person_character))
    (set `/Game/FirstPerson/Blueprints/BP_FirstPersonCharacter.Health` (- _health 1.0) _asbp_first_person_character)
    (if (<= _health 0.0)
      (bind _returnvalue_2 (`|CreateWidget` "/Game/Blueprints/UMG/WBP_Death.WBP_Death_C" _returnvalue))
      (`UserWidget.AddToViewport` _returnvalue_2 0)
      (`WidgetBlueprintLibrary.SetInputMode_UIOnlyEx` _returnvalue _returnvalue_2)
      (set `PlayerController.bShowMouseCursor` true _returnvalue)
      (else
        (`KismetSystemLibrary.Delay` 3.0)
        (`/Engine/EditorBlueprintResources/StandardMacros.IsValid` _asbp_first_person_character
          (:`Is Valid`
            (bind _output_get (set `/Game/FirstPerson/Blueprints/BP_FirstPersonCharacter.Health` (- (`/Game/FirstPerson/Blueprints/BP_FirstPersonCharacter.Health` _asbp_first_person_character) 1.0) _asbp_first_person_character))
            (`KismetSystemLibrary.PrintString` (`KismetStringLibrary.Conv_DoubleToString` _output_get))))))))

(fn `UserConstructionScript`)