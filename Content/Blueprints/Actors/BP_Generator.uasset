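; BP_Generator is an interactable generator that temporarily powers the gas panel and steadies point lamps once the player has a charger.
; Interacting while inactive swaps the Charger mesh material, stops lamp flickering and starts a looping one-second timer.
; Each tick flags BP_Gas_Panel as electrified, rotates the blade and raises Power up to MaxPower.
; At MaxTime it cuts panel power, stops its fan, restarts flickering and resets.
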(event `/Game/Blueprints/Interaction/BP_InteractionIF.InteractWith`
  (params (PC :type "/Game/FirstPerson/Blueprints/BP_FirstPersonCharacter Object Reference"))
  (bind _asbp_first_person_character (cast `/Game/FirstPerson/Blueprints/BP_FirstPersonCharacter` (`GameplayStatics.GetPlayerCharacter` 0)))
  (if (`self.IsActive`)
    _
    (elif (`/Game/FirstPerson/Blueprints/BP_FirstPersonCharacter.HasCharger` _asbp_first_person_character)
      (`self.InsertCharger`)
      (`self.StartCharge`))))

(event `StartCharge`
  (set `self.IsActive` true)
  (bind _outactors (`GameplayStatics.GetAllActorsOfClass` "/Game/Blueprints/Actors/BP_PointLamp.BP_PointLamp_C"))
  (for _index (range -1 (+ (`KismetArrayLibrary.Array_Length` _outactors) 1))
    (`/Game/Blueprints/Actors/BP_PointLamp.StopFlickering` (`|GetArrayItem` _outactors _index)))
  (`KismetSystemLibrary.K2_SetTimerDelegate` (delegate `Charge`) 1.0 true))

(event `Charge`
  (bind _power (`self.Power`))
  (bind _generatorblade (`self.GeneratorBlade`))
  (bind (_relativerotation_roll _relativerotation_pitch _relativerotation_yaw) (`KismetMathLibrary.BreakRotator` (`SceneComponent.RelativeRotation` _generatorblade)))
  (bind _returnvalue (`GameplayStatics.GetActorOfClass` "/Game/Seamus_MEGJAM_Stuff/Gas_Panel/BP_Gas_Panel.BP_Gas_Panel_C"))
  (set `/Game/Seamus_MEGJAM_Stuff/Gas_Panel/BP_Gas_Panel.HasLec` true _returnvalue)
  (bind _output_get (set `self.Relative Rotation Y (Pitch)` _relativerotation_pitch))
  (`SceneComponent.K2_SetRelativeRotation` _generatorblade (`KismetMathLibrary.MakeRotator` _relativerotation_roll (+ _output_get 10.0) _relativerotation_yaw) false false)
  (bind _output_get_2 (set `self.Time` (+ (`self.Time`) 1.0)))
  (if (<= (`self.MaxTime`) _output_get_2)
    (`self.StopCharge`)
    (set `/Game/Blueprints/Actors/BP_PointLamp.IsStopped` false (`|GetArrayItem` (stale `StartCharge` _outactors) (stale `StartCharge` _index)))
    (elif (not (<= (`self.MaxPower`) _power))
      (set `self.Power` (+ _power 10.0)))))

(event `StopCharge`
  (set `/Game/Seamus_MEGJAM_Stuff/Gas_Panel/BP_Gas_Panel.HasLec` false (stale `Charge` _returnvalue))
  (`/Game/Seamus_MEGJAM_Stuff/Gas_Panel/BP_Gas_Panel.StopFan` (stale `Charge` _returnvalue))
  (bind _outactors (`GameplayStatics.GetAllActorsOfClass` "/Game/Blueprints/Actors/BP_PointLamp.BP_PointLamp_C"))
  (for (_ _array_index) _outactors
    (`/Game/Blueprints/Actors/BP_PointLamp.StartFlickering` (`|GetArrayItem` _outactors _array_index)))
  (set `self.Time` 0.0)
  (set `self.IsActive` false)
  (set `self.Power` 0.0))

(event `InsertCharger`
  (`PrimitiveComponent.SetMaterial` (`self.Charger`) 0 "/Game/Seamus_MEGJAM_Stuff/Generator/Lever.Lever"))

(fn `LookAt`
  (returns (Message :type Text) (Player :type "/Game/FirstPerson/Blueprints/BP_FirstPersonCharacter Object Reference"))
  (return "Interact" null))

(fn `UserConstructionScript`)