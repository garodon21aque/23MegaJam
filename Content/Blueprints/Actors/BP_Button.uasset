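; BP_Button is an interactable button that opens and closes a linked BP_Door.
; On interaction, if usable, it casts its InteractActor to BP_Door, toggles the door based on its open state and swaps the button material to match.
; LookAt supplies the "Open/Close [E]" prompt text, while Tick calls it without using the result and has an empty CanBeUsed branch.
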(event `self.ReceiveTick`
  (params (DeltaSeconds :type "Float (single-precision)"))
  (`self.LookAt`)
  (if (`self.CanBeUsed`)
    _))

(event `self.InteractWith`
  (params (PC :type "/Game/FirstPerson/Blueprints/BP_FirstPersonCharacter Object Reference"))
  (bind _button (`self.Button`))
  (if (`self.CanBeUsed`)
    (bind _asbp_door (cast `/Game/Blueprints/Actors/BP_Door` (`self.InteractActor`)))
    (`/Engine/EditorBlueprintResources/StandardMacros.IsValid` _asbp_door
      (:`Is Valid`
        (if (`/Game/Blueprints/Actors/BP_Door.IsOpen` _asbp_door)
          (`PrimitiveComponent.SetMaterial` _button 0 "/AnimationSharing/AnimSharingRed.AnimSharingRed")
          (`/Game/Blueprints/Actors/BP_Door.CloseDoor` _asbp_door)
          (else
            (`PrimitiveComponent.SetMaterial` _button 0 "/Game/Seamus_Stuff/Gas_Panel(Real)/M_Button1.M_Button1")
            (`/Game/Blueprints/Actors/BP_Door.OpenDoor` _asbp_door)))))))

(fn `LookAt`
  (returns (Message :type Text) (Player :type "/Game/FirstPerson/Blueprints/BP_FirstPersonCharacter Object Reference"))
  (return "Open/Close [E]" null))

(fn `UserConstructionScript`)