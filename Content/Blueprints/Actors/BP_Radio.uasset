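; BP_Radio is an interactable radio that serves as the rescue objective and decides the win or death ending.
; Interacting repairs it if the player has the cog, starts the GameMode rescue countdown, and, once repaired, plays FMOD radio audio.
; With the antenna, it swaps mesh and stops the generator's charge.
; Overlapping FinisGame then shows the win screen if the timer has expired, otherwise a monster death sequence.
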(event `Repair`
  (`FMODBlueprintStatics.EventInstanceSetParameter` (stale `TurnOn` _returnvalue) "Interactable" 2.0)
  (bind _asbp_first_person_character (cast `/Game/FirstPerson/Blueprints/BP_FirstPersonCharacter` (`GameplayStatics.GetPlayerCharacter` 0)))
  (if (`/Game/FirstPerson/Blueprints/BP_FirstPersonCharacter.HasCog` _asbp_first_person_character)
    (set `self.IsRepaired` true)))

(event `TurnOn`
  (bind _isrepaired (`self.IsRepaired`))
  (bind _asbp_player_controller (cast `/Game/Blueprints/Player/BP_PlayerController` (`GameplayStatics.GetPlayerController` 0)))
  (bind _asbp_first_person_game_mode (cast `/Game/FirstPerson/Blueprints/BP_FirstPersonGameMode` (`GameplayStatics.GetGameMode`)))
  (`/Game/FirstPerson/Blueprints/BP_FirstPersonGameMode.Start Timer CountDown` _asbp_first_person_game_mode)
  (`Widget.SetVisibility` (`/Game/Blueprints/UMG/WBP_HUD.RescueTime` (`/Game/Blueprints/Player/BP_PlayerController.HUd` _asbp_player_controller)) "Visible")
  (if _isrepaired
    (bind _returnvalue (`FMODBlueprintStatics.PlayEventAtLocation` "/Game/FMOD/Events/Interactable/Interactable_Radio.Interactable_Radio" (`self.GetTransform`) _isrepaired))
    (`FMODBlueprintStatics.EventInstanceSetParameter` _returnvalue "Interactable" 1.0)
    (if (`/Game/FirstPerson/Blueprints/BP_FirstPersonCharacter.HasAntenna` (stale `Repair` _asbp_first_person_character))
      (set `self.HasAntenna` true)
      (`self.TurnOFFLEC`)
      (`StaticMeshComponent.SetStaticMesh` (`self.StaticMesh`) (`self.AntennaMEsh`)))))

(event `self.FinisGame.OnComponentBeginOverlap`
  (params (OverlappedComponent :type "PrimitiveComponent Object Reference") (OtherActor :type "Actor Object Reference") (OtherComp :type "PrimitiveComponent Object Reference") (OtherBodyIndex :type Integer) (bFromSweep :type Boolean) (SweepResult :type "HitResult Structure (by ref)"))
  (bind _returnvalue (`GameplayStatics.GetPlayerController` 0))
  (bind _asbp_first_person_character (cast `/Game/FirstPerson/Blueprints/BP_FirstPersonCharacter` OtherActor))
  (`/Engine/EditorBlueprintResources/StandardMacros.IsValid` _asbp_first_person_character
    (:`Is Valid`
      (if (`self.HasAntenna`)
        (`FMODBlueprintStatics.PlayEvent2D` "/Game/FMOD/Events/Interactable/Interactable_Correct.Interactable_Correct")
        (bind _asbp_first_person_game_mode (cast `/Game/FirstPerson/Blueprints/BP_FirstPersonGameMode` (`GameplayStatics.GetGameMode`)))
        (if (<= (`/Game/FirstPerson/Blueprints/BP_FirstPersonGameMode.Timer` _asbp_first_person_game_mode) 0)
          (bind _returnvalue_2 (`|CreateWidget` "/Game/Blueprints/UMG/WBP_Win.WBP_Win_C" _returnvalue))
          (`UserWidget.AddToViewport` _returnvalue_2 0)
          (`WidgetBlueprintLibrary.SetInputMode_UIOnlyEx` _returnvalue _returnvalue_2)
          (set `PlayerController.bShowMouseCursor` true _returnvalue)
          (else
            (bind _returnvalue_3 (`FMODBlueprintStatics.PlayEvent2D` "/Game/FMOD/Events/Monster/Monster_DeathSequence.Monster_DeathSequence"))
            (`KismetSystemLibrary.Delay` 8.0)
            (`PrimitiveComponent.SetCollisionProfileName` (`/Game/FirstPerson/Blueprints/BP_FirstPersonCharacter.FirstPersonMesh` (stale `Repair` _asbp_first_person_character)) "Ragdoll" true)
            (`KismetSystemLibrary.Delay` 3.0)
            (bind _returnvalue_4 (`|CreateWidget` "/Game/Blueprints/UMG/WBP_Death.WBP_Death_C" _returnvalue))
            (`FMODBlueprintStatics.EventInstanceStop` _returnvalue_3 true)
            (`UserWidget.AddToViewport` _returnvalue_4 0)
            (`WidgetBlueprintLibrary.SetInputMode_UIOnlyEx` _returnvalue _returnvalue_4)
            (set `PlayerController.bShowMouseCursor` true _returnvalue)))
        (else
          (`FMODBlueprintStatics.PlayEvent2D` "/Game/FMOD/Events/Interactable/Interactable_Incorrect.Interactable_Incorrect"))))))

(event `/Game/Blueprints/Interaction/BP_InteractionIF.InteractWith`
  (params (PC :type "/Game/FirstPerson/Blueprints/BP_FirstPersonCharacter Object Reference"))
  (`self.Repair`)
  (`self.TurnOn`))

(fn `LookAt`
  (returns (Message :type Text) (Player :type "/Game/FirstPerson/Blueprints/BP_FirstPersonCharacter Object Reference"))
  (if (`self.IsRepaired`)
    (if (`self.HasAntenna`)
      (bind _output_get (set `self.Current` (`self.TurnONTXT`)))
      (return _output_get null)
      (else
        (bind _output_get_2 (set `self.Current` (`self.AntennaTXT`)))
        (return _output_get_2 null)))
    (else
      (bind _output_get_3 (set `self.Current` (`self.RepairTXT`)))
      (return _output_get_3 null))))

(fn `TurnOFFLEC`
  (bind _returnvalue (`GameplayStatics.GetActorOfClass` "/Game/Blueprints/Actors/BP_Generator.BP_Generator_C"))
  (`/Game/Blueprints/Actors/BP_Generator.StopCharge` _returnvalue))

(fn `UserConstructionScript`)