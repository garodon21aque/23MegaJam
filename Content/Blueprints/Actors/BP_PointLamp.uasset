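; Point lamp actor that flickers at random from BeginPlay by briefly switching off its Lamp and RectLight components.
; A looping timer calls Flickering, which uses random Delays to wait a few seconds, cut both intensities to zero, then restore them.
; StopFlickering sets both lights to a brighter intensity but does not clear the timer or pending delays.
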(event `self.ReceiveBeginPlay`
  (`self.StartFlickering`))

(event `StartFlickering`
  (`KismetSystemLibrary.K2_SetTimerDelegate` (delegate `Flickering`) 1.5 true))

(event `Flickering`
  (`KismetSystemLibrary.Delay` (`KismetMathLibrary.RandomFloatInRange` 4.0 6.0))
  (`LightComponent.SetIntensity` (`self.Lamp`) 0.0)
  (`LightComponent.SetIntensity` (`self.RectLight`) 0.0)
  (`KismetSystemLibrary.Delay` (`KismetMathLibrary.RandomFloatInRange` 0.1 1.0))
  (`LightComponent.SetIntensity` (`self.Lamp`) 500.0)
  (`LightComponent.SetIntensity` (`self.RectLight`) 500.0))

(event `StopFlickering`
  (`LightComponent.SetIntensity` (`self.Lamp`) 1000.0)
  (`LightComponent.SetIntensity` (`self.RectLight`) 1000.0))

(fn `UserConstructionScript`)